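; Ball actor for a paddle game, moved entirely by setting the physics linear velocity of its static mesh.
; BeginPlay launches it along +Y at a fixed speed.
; On overlap with a RightPaddle it reverses Y, keeps Z, and sets X to the paddle's X velocity plus a random offset.
; Overlaps with any other actor are ignored.
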(event EventBeginPlay
  ;[1 1 1] Initialize Ball Velocity
  (Physics|SetPhysicsLinearVelocity (Variables|Default|GetStaticMesh) "0,2000.000000, 0" false "None"))

(event Collision|EventActorBeginOverlap
  (params (OtherActor :type Actor%20Object%20Reference))
  ;[1 1 1] Player 1 Paddle Collision
  (bind _asright_paddle (Utilities|Casting|CastToRightPaddle OtherActor))
  ;;[1 1 1] Calculate X Value from paddle X and randomness
  (bind _returnvalue (Physics|GetPhysicsLinearVelocity (Variables|/Game/Blueprints/Pawns/RightPaddle.RightPaddle_C|GetPaddleMesh _asright_paddle) "None"))
  ;;[1 1 1] Reverse Y
  (bind _returnvalue_2 (Physics|GetPhysicsLinearVelocity (Variables|Default|GetStaticMesh) "None"))
  ;;[1 1 1] Set New Velocity
  (Physics|SetPhysicsLinearVelocity (Variables|Default|GetStaticMesh) (Math|Vector|MakeVector (+ (.X (Math|Vector|BreakVector _returnvalue)) (Math|Random|RandomFloatinRange -1e+03 1e+03)) (* (.Y (Math|Vector|BreakVector _returnvalue_2)) -1.0) (.Z (Math|Vector|BreakVector _returnvalue_2))) false "None"))

(event EventTick
  (params (DeltaSeconds :type Float%20%28single-precision%29)))

(fn ConstructionScript)