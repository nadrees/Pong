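; EnemyPaddle is an AI-controlled paddle that follows Ball actors along the X axis.
; Each tick it finds every Ball and pushes its static mesh with an impulse from the clamped X offset, scaled by Speed.
; If the paddle passes either fixed X limit, it is teleported just inside that bound instead of receiving the impulse.
; The impulse is not scaled by delta time.
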(event EventBeginPlay)

(event Collision|EventActorBeginOverlap
  (params (OtherActor :type Actor%20Object%20Reference)))

(event EventTick
  (params (DeltaSeconds :type Float%20%28single-precision%29))
  (bind _returnvalue (Transformation|GetActorLocation))
  (bind (_x _y _z) (Math|Vector|BreakVector _returnvalue))
  ;[1 1 1] AI Paddle
  (bind _outactors (Actor|GetAllActorsOfClass "/Game/Blueprints/Actors/Ball.Ball_C"))
  (for _array_element _outactors
    ;;[1 1 1] Clamp Max X Height
    (if (> _x 1.5e+03)
      (Transformation|SetActorLocation (Math|Vector|MakeVector 1499.0 _y _z) false)
      (else
        ;;[1 1 1] Clamp Min X Height
        (if (< _x -1.5e+03)
          (Transformation|SetActorLocation (Math|Vector|MakeVector -1499.0 _y _z) false)
          (else
            ;;[1 1 1] Move Paddle
            (Physics|AddImpulse (Variables|Default|GetStaticMesh) (* (Math|Vector|MakeVector (Math|Float|Clamp(Float) (- (.X (Math|Vector|BreakVector (Transformation|GetActorLocation _array_element))) (.X (Math|Vector|BreakVector (Transformation|GetActorLocation)))) -1e+01 1e+01) 0.0 0.0) (Variables|Default|GetSpeed)) "None" false)))))))

(fn ConstructionScript)