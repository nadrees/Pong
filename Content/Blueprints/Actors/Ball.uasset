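; Pong ball actor that bounces between paddles and walls, keeps both players' scores and ends the match.
; Overlap casts pick the response: paddles reverse Y and set X from paddle velocity plus randomness, while horizontal boundaries reverse X.
; Goals recenter and relaunch the ball, then update the score via tagged TextRender components.
; When a score reaches WinScore, it prints the winner, stops the ball and opens P1_Main after a delay.
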(event EventBeginPlay
  ;[1 1 1] Initialize Ball Velocity
  (Physics|SetPhysicsLinearVelocity (Variables|Default|GetStaticMesh) "0,2000.000000, 0" false "None"))

(event Collision|EventActorBeginOverlap
  (params (OtherActor :type Actor%20Object%20Reference))
  ;[1 1 1] Player 1 Paddle Collision
  (bind _asright_paddle (Utilities|Casting|CastToRightPaddle OtherActor)
    (:then
      (CallFunction|HandlePaddleCollision (Variables|/Game/Blueprints/Pawns/RightPaddle.RightPaddle_C|GetPaddleMesh _asright_paddle))
      (Audio|PlaySoundatLocation "/Game/Sounds/S_ballCollision.S_ballCollision" "0, 0, 0" :!label _label))
    (:CastFailed
      ;[1 1 1] AI Paddle Collision
      (bind _asenemy_paddle (Utilities|Casting|CastToEnemyPaddle OtherActor)
        (:then
          (CallFunction|HandlePaddleCollision (Variables|/Game/Blueprints/Actors/EnemyPaddle.EnemyPaddle_C|GetStaticMesh _asenemy_paddle))
          (goto _label))
        (:CastFailed
          ;[1 1 1] Wall Collision
          (Utilities|Casting|CastToHorizontalBoundary OtherActor
            (:then
              (bind _returnvalue (Physics|GetPhysicsLinearVelocity (Variables|Default|GetStaticMesh) "None"))
              (Physics|SetPhysicsLinearVelocity (Variables|Default|GetStaticMesh) (Math|Vector|MakeVector (* (.X (Math|Vector|BreakVector _returnvalue)) -1.0) (.Y (Math|Vector|BreakVector _returnvalue)) (.Z (Math|Vector|BreakVector _returnvalue))) false "None")
              (goto _label))
            (:CastFailed
              ;[1 1 1] Goals Collision
              (Utilities|Casting|CastToLeftGoal OtherActor
                (:then
                  (CallFunction|HandleGoalCollision 2e+03 false))
                (:CastFailed
                  (Utilities|Casting|CastToRightGoal OtherActor)
                  (CallFunction|HandleGoalCollision -2e+03 true)))
              (Audio|PlaySoundatLocation "/Game/Sounds/S_ballGoal.S_ballGoal" "0, 0, 0")
              (CallFunction|CheckEndGame)
              ;;[1 1 1] End Game
              (if (Variables|Default|GetGameOver)
                (Physics|SetPhysicsLinearVelocity (Variables|Default|GetStaticMesh) "0, 0, 0" false "None")
                (Utilities|FlowControl|Delay 3.0)
                (Game|OpenLevel(byName) "P1_Main")))))))))

(event EventTick
  (params (DeltaSeconds :type Float%20%28single-precision%29)))

(fn ConstructionScript)

(fn HandlePaddleCollision
  (params (Paddle%20Static%20Mesh%20Component :type Static%20Mesh%20Component%20Object%20Reference))
  ;[1 1 1] Calculate X Value from paddle X and randomness
  (bind _returnvalue (Physics|GetPhysicsLinearVelocity Paddle%20Static%20Mesh%20Component "None"))
  ;[1 1 1] Reverse Y
  (bind _returnvalue_2 (Physics|GetPhysicsLinearVelocity (Variables|Default|GetStaticMesh) "None"))
  ;[1 1 1] Set New Velocity
  (Physics|SetPhysicsLinearVelocity (Variables|Default|GetStaticMesh) (Math|Vector|MakeVector (+ (.X (Math|Vector|BreakVector _returnvalue)) (Math|Random|RandomFloatinRange -1e+03 1e+03)) (* (.Y (Math|Vector|BreakVector _returnvalue_2)) -1.0) (.Z (Math|Vector|BreakVector _returnvalue_2))) false "None"))

(fn HandleGoalCollision
  (params (NewVelY :type Float%20%28single-precision%29) (IncrementLPlayerScore :type Boolean))
  ;[1 1 1] Reset Ball
  (Transformation|SetActorLocation "0,0.000000, 0" false)
  (Physics|SetPhysicsLinearVelocity (Variables|Default|GetStaticMesh) (Math|Vector|MakeVector 0.0 NewVelY 0.0) false "None")
  ;[1 1 1] Update Score
  (if IncrementLPlayerScore
    (bind _output_get (Variables|Default|SetLPlayer_Score (+ (Variables|Default|GetLPlayer_Score) 1)))
    (CallFunction|SetScoreText "LPlayer_Score" _output_get)
    (else
      (bind _output_get_2 (Variables|Default|SetRPlayer_Score (+ (Variables|Default|GetRPlayer_Score) 1)))
      (CallFunction|SetScoreText "RPlayer_Score" _output_get_2))))

(fn SetScoreText
  (params (Tag%20Name :type String) (Score :type Integer))
  (bind _outactors (Actor|GetAllActorsOfClass "/Script/Engine.TextRenderActor"))
  (for _array_element _outactors
    (if (Components|ComponentHasTag (Variables|/Script/Engine.TextRenderActor|GetTextRender _array_element) (Utilities|String|StringToName Tag%20Name))
      (Rendering|Components|TextRender|SetText (Variables|/Script/Engine.TextRenderActor|GetTextRender _array_element) (Utilities|Text|ToText(Integer) Score)))))

(fn CheckEndGame
  (bind _win_score (Variables|Default|GetWin_Score))
  (bind _returnvalue (- _win_score 1))
  ;[1 1 1] Left Player Win Conditions
  (if (> (Math|Conversions|ToFloat(Integer) (Variables|Default|GetLPlayer_Score)) (Math|Conversions|ToFloat(Integer) _returnvalue))
    (Development|PrintString "Left Player Wins!")
    (Variables|Default|SetGameOver true :!label _label)
    (else
      ;[1 1 1] Right Player Win Conditions
      (if (> (Math|Conversions|ToFloat(Integer) (Variables|Default|GetRPlayer_Score)) (Math|Conversions|ToFloat(Integer) _returnvalue))
        (Development|PrintString "Right Player Wins!")
        (goto _label)))))