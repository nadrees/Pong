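; RightPaddle is the pawn for the right-hand paddle, moved along world X by the P2_Vertical input axis.
; Each tick it applies a force to PaddleMesh scaled by the axis value and Speed.
; When the actor passes MaxX or MinX, it is instead teleported one unit back inside that bound, without sweep, and receives no force that frame.
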(event EventBeginPlay)

(event Collision|EventActorBeginOverlap
  (params (OtherActor :type Actor%20Object%20Reference)))

(event EventTick
  (params (DeltaSeconds :type Float%20%28single-precision%29))
  (bind _returnvalue (Transformation|GetActorLocation))
  (bind _maxx (Variables|Default|GetMaxX))
  (bind _minx (Variables|Default|GetMinX))
  (bind (_x _y _z) (Math|Vector|BreakVector _returnvalue))
  (bind (_x_2 _y_2 _z_2) (Math|Vector|BreakVector _returnvalue))
  ;[1 1 1] Move Paddle
  ;;[1 1 1] Clamp Max Height
  (if (> (.X (Math|Vector|BreakVector _returnvalue)) _maxx)
    (Transformation|SetActorLocation (Math|Vector|MakeVector (- _maxx 1.0) _y_2 _z_2) false)
    (else
      ;;[1 1 1] Clamp Min Height
      (if (< (.X (Math|Vector|BreakVector _returnvalue)) _minx)
        (Transformation|SetActorLocation (Math|Vector|MakeVector (+ _minx 1.0) _y _z) false)
        (else
          (Physics|AddForce (Variables|Default|GetPaddleMesh) (Math|Vector|MakeVector (* (Input|AxisValues|GetP2_Vertical) (Variables|Default|GetSpeed)) 0.0 0.0) "None" false))))))

(fn ConstructionScript)